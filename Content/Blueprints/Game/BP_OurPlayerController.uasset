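; Player controller that routes mouse wheel and gamepad input to in-world info screens and the pause menu.
; Scroll input reaches the focused WB_InfoFrame when CharacterOnButton is set; Escape or P toggles pause, input mode and cursor.
; It also animates highscore gains via a timeline, flags the ending and stops interaction tracing.
; BeginPlay schedules a delayed BP_Kai spawn with animation and video, and holding T fast-forwards time.
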(event `InteractController`
  (`self.CheckPauseControllerInteract`))

(event `ControllerCross`
  (params (Direction :type "/Game/Blueprints/Game/E_ControllerCross Enum" :default "NewEnumerator0"))
  (bind _returnvalue (and (`self.CharacterOnButton`) (`KismetSystemLibrary.IsValid` (`self.CurrentlyFocusedScreen`))))
  (`self.CheckPauseControllerInput` Direction)
  (switch `/Game/Blueprints/Game/E_ControllerCross` Direction
    (:`NewEnumerator0`
      (`|ExecutionSequence`
        (:`then_0`
          (if _returnvalue :!label _label
            (bind _aswb_info_frame (cast `/Game/Blueprints/Game/WB_InfoFrame` (`WidgetComponent.GetWidget` (`self.CurrentlyFocusedScreen`))))
            (`/Game/Blueprints/Game/WB_InfoFrame.ScrollInput` _aswb_info_frame true)))))
    (:`NewEnumerator1`
      (`|ExecutionSequence`
        (:`then_0`
          (if _returnvalue :!label _label_2
            (bind _aswb_info_frame_2 (cast `/Game/Blueprints/Game/WB_InfoFrame` (`WidgetComponent.GetWidget` (`self.CurrentlyFocusedScreen`))))
            (`/Game/Blueprints/Game/WB_InfoFrame.ScrollInput` _aswb_info_frame_2 false)))))))

(event `Key|MouseScrollUp`
  (params (Key :type "Key Structure"))
  (:`Pressed`
    (goto _label)))

(event `Key|MouseScrollDown`
  (params (Key :type "Key Structure"))
  (:`Pressed`
    (goto _label_2)))

(event `self.ReceiveBeginPlay`
  (set `self.bShowMouseCursor` false)
  (`WidgetBlueprintLibrary.SetInputMode_GameOnly` self)
  (bind _returnvalue (`GameplayStatics.GetActorOfClass` "/Game/Blueprints/Game/BP_CameraHead.BP_CameraHead_C"))
  (set `self.CamHeadRef` _returnvalue)
  (`KismetSystemLibrary.ExecuteConsoleCommand` "DISABLEALLSCREENMESSAGES" null)
  (`KismetSystemLibrary.Delay` 17.0)
  (`self.SpawnKAI` 10.0 10.0))

(event `Key|T`
  (params (Key :type "Key Structure"))
  (:`Pressed`
    (`GameplayStatics.SetGlobalTimeDilation` 60.0))
  (:`Released`
    (`GameplayStatics.SetGlobalTimeDilation` 1.0)))

(event `Key|Escape` :paused true
  (params (Key :type "Key Structure"))
  (:`Pressed`
    (`self.TogglePause` :!label _label_3)))

(event `Key|P` :paused true
  (params (Key :type "Key Structure"))
  (:`Pressed`
    (goto _label_3)))

(event `AddPointsToHighscore`
  (params (Duration :type "Float (double-precision)") (PointsToAdd :type Integer))
  (`TimelineComponent.SetPlayRate` (`self.AddPoints`) (/ 1.0 Duration))
  (set `self.HighscoreBefore` (`KismetMathLibrary.Conv_IntToDouble` (`self.CurrentHighscore`)))
  (set `self.HighscoreTarget` (+ PointsToAdd (`self.CurrentHighscore`)))
  (bind (_direction _newtrack_0) (`Timeline|AddPoints` :!via `PlayFromStart`)
    (:`Update`
      (set `self.CurrentHighscore` (`KismetMathLibrary.FTrunc` (`KismetMathLibrary.Lerp` (`self.HighscoreBefore`) (`self.HighscoreTarget`) _newtrack_0)))
      (`/Game/UI/Game/WB_HighScore.UpdatePoints` (`/Game/UI/Game/WB_UI.WB_HighScore` (`self.UI`)) (`self.CurrentHighscore`)))))

(event `SpawnKAI`
  (params (RolloutAfterTime :type "Float (double-precision)") (StartVideo :type "Float (single-precision)"))
  (bind _returnvalue (`|SpawnActorFromClass` "/Game/Lewin/BP_Kai.BP_Kai_C" (`KismetMathLibrary.MakeTransform` (845.225342 -14.426919 2492.47876)) "Undefined" "OverrideRootScale" null null))
  (`|ExecutionSequence`
    (:`then_0`
      (`KismetSystemLibrary.Delay` RolloutAfterTime)
      (`/Game/Lewin/BP_Kai.Animate` _returnvalue))
    (:`then_1`
      (`KismetSystemLibrary.Delay` StartVideo)
      (`/Game/Lewin/BP_Kai.PlayVideo` _returnvalue))))

(fn `CheckPauseControllerInput`
  (params (Direction :type "/Game/Blueprints/Game/E_ControllerCross Enum" :default "NewEnumerator0"))
  (if (`self.InPauseMenu`)
    (`/Game/UI/Game/WB_PauseMenu.ControllerCross` (`/Game/UI/Game/WB_UI.WB_PauseMenu_46` (`self.UI`)) Direction)))

(fn `CheckPauseControllerInteract`
  (if (`self.InPauseMenu`)
    (`/Game/UI/Game/WB_PauseMenu.SelectNewIndexNew` (`/Game/UI/Game/WB_UI.WB_PauseMenu_46` (`self.UI`)) 0 -1 true)))

(fn `DefaultGraphicsSettings`
  (bind _returnvalue (`GameUserSettings.GetGameUserSettings`))
  (`GameUserSettings.SetDynamicResolutionEnabled` _returnvalue true)
  (`GameUserSettings.ApplySettings` _returnvalue false))

(fn `TogglePause`
  (bind _output_get (set `self.InPauseMenu` (not (`GameplayStatics.IsGamePaused`))))
  (`GameplayStatics.SetGamePaused` _output_get)
  (if (`self.InPauseMenu`)
    (`/Game/UI/Game/WB_UI.ShowPauseMenu` (`self.UI`) true)
    (`WidgetBlueprintLibrary.SetInputMode_GameAndUIEx` self null "DoNotLock" false)
    (set `self.bShowMouseCursor` true)
    (else
      (`/Game/UI/Game/WB_UI.ShowPauseMenu` (`self.UI`) false)
      (set `self.bShowMouseCursor` false)
      (`WidgetBlueprintLibrary.SetInputMode_GameOnly` self))))

(fn `TriggerEnd`
  (set `self.WON_FinalCutscene` true)
  (set `/Game/Interaction/AC_InteractionTrace.StopTracing` true (`/Game/Blueprints/Game/BP_FirstPersonCharacter.AC_InteractionTrace` (`/Game/Blueprints/Game/BP_GeneralFunctions.GetCharacterRef`))))

(fn `TriggerFinalCutsceneInfoPoint`)

(fn `UpdateUsingController`
  (params (ControllerInput :type Boolean))
  (bind _currentlyfocusedscreen (`self.CurrentlyFocusedScreen`))
  (set `self.ControllerInput` ControllerInput)
  (`/Engine/EditorBlueprintResources/StandardMacros.IsValid` _currentlyfocusedscreen
    (:`Is Valid`
      (bind _aswb_info_frame (cast `/Game/Blueprints/Game/WB_InfoFrame` (`WidgetComponent.GetWidget` _currentlyfocusedscreen)))
      (if (`/Game/Blueprints/Game/WB_InfoFrame.Scrollable` _aswb_info_frame)
        (`/Game/Blueprints/Game/WB_InfoFrame.ShowScrollInfo` _aswb_info_frame true)))))

(fn `UserConstructionScript`)