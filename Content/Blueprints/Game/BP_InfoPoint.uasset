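; BP_InfoPoint is a pressure-plate info station that reveals floating info widgets while a character stands on it.
; Trigger overlaps drive a timeline that sinks and raises the button, and show or hide the WB_InfoFrame widgets under InfoPoints with staggered delays.
; CheckForInfo finds a frame by component tag, calls UnlockedInfo on it, and can turn the matching light mesh and point light green after a delay.
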(event `self.ReceiveBeginPlay`
  ;[1 1 1] Event Begin Play
  (set `self.InitialRelativeButtonLoc` (`SceneComponent.RelativeLocation` (`self.Button`))))

(event `PlayPressureAnimation`
  (params (enter :type Boolean))
  (bind _z (.z (`self.InitialRelativeButtonLoc`)))
  ;[1 1 1] Animation
  (if enter
    (if (not (`self.ButtonAnimationButtonPressed`))
      (set `self.ButtonAnimationButtonPressed` true)
      (bind (_direction _newtrack_0) (`Timeline|PressurePlate` :!label _label)
        (:`Update`
          (`SceneComponent.K2_SetRelativeLocation` (`self.Button`) (`KismetMathLibrary.MakeVector` (.x (`self.InitialRelativeButtonLoc`)) (.y (`self.InitialRelativeButtonLoc`)) (`KismetMathLibrary.Lerp` _z (- _z 12.0) _newtrack_0)) false false))))
    (else
      (set `self.ButtonAnimationButtonPressed` false)
      (goto _label :!via `Reverse`))))

(event `self.TriggerPlate.OnComponentBeginOverlap`
  (params (OverlappedComponent :type "PrimitiveComponent Object Reference") (OtherActor :type "Actor Object Reference") (OtherComp :type "PrimitiveComponent Object Reference") (OtherBodyIndex :type Integer) (bFromSweep :type Boolean) (SweepResult :type "HitResult Structure (by ref)"))
  ;[1 1 1] Trigger Zone Button
  (`self.PlayPressureAnimation` true)
  (if (<= (`KismetArrayLibrary.Array_Length` (`PrimitiveComponent.GetOverlappingActors` (`self.TriggerPlate`) "/Script/Engine.Character")) 1)
    (`self.Show`)))

(event `self.TriggerPlate.OnComponentEndOverlap`
  (params (OverlappedComponent :type "PrimitiveComponent Object Reference") (OtherActor :type "Actor Object Reference") (OtherComp :type "PrimitiveComponent Object Reference") (OtherBodyIndex :type Integer))
  ;[1 1 1] Trigger Zone Button
  (if (== (`KismetArrayLibrary.Array_Length` (`PrimitiveComponent.GetOverlappingActors` (`self.TriggerPlate`) "/Script/Engine.Character")) 0)
    (`self.PlayPressureAnimation` false)
    (`self.Hide`)))

(event `Show`
  ;[1 1 1] Show and Hide screen content
  (for (_array_element _array_index) (`SceneComponent.GetChildrenComponents` (`self.InfoPoints`) true)
    (bind _aswidget_component (cast `WidgetComponent` _array_element))
    (bind _aswb_info_frame (cast `/Game/Blueprints/Game/WB_InfoFrame` (`WidgetComponent.GetWidget` _aswidget_component)))
    (`/Game/Blueprints/Game/WB_InfoFrame.PlayShow` _aswb_info_frame true (* (`KismetMathLibrary.Conv_IntToDouble` _array_index) 0.2))))

(event `Hide`
  ;[1 1 1] Show and Hide screen content
  (for (_array_element _array_index) (`SceneComponent.GetChildrenComponents` (`self.InfoPoints`) true)
    (bind _aswidget_component (cast `WidgetComponent` _array_element))
    (bind _aswb_info_frame (cast `/Game/Blueprints/Game/WB_InfoFrame` (`WidgetComponent.GetWidget` _aswidget_component)))
    (`/Game/Blueprints/Game/WB_InfoFrame.PlayShow` _aswb_info_frame false (* (`KismetMathLibrary.Conv_IntToDouble` _array_index) 0.1))))

(event `CheckForInfo`
  (params (TagID :type Name) (TurnOnLightAfterTime :type Boolean) (AfterTime :type "Float (double-precision)"))
  ;[1 1 1] Check for Info
  (bind _aswb_info_frame (`self.ScanTag` TagID))
  (`/Game/Blueprints/Game/WB_InfoFrame.UnlockedInfo` _aswb_info_frame TagID)
  ;[1 1 1] Turn On Light after certain duration
  (if TurnOnLightAfterTime
    (`KismetSystemLibrary.Delay` AfterTime)
    (`self.TurnLightGreenByTag` TagID)))

(fn `ScanTag`
  (params (ID :type Name))
  (returns (`AsWB Info Frame` :type "/Game/Blueprints/Game/WB_InfoFrame Object Reference"))
  (for _array_element (`SceneComponent.GetChildrenComponents` (`self.InfoPoints`) false)
    (bind _returnvalue (`SceneComponent.GetChildComponent` _array_element 0))
    (if (== (`|GetArrayItem` (`ActorComponent.ComponentTags` _returnvalue)) ID)
      (bind _aswidget_component (cast `WidgetComponent` _returnvalue))
      (bind _aswb_info_frame (cast `/Game/Blueprints/Game/WB_InfoFrame` (`WidgetComponent.GetWidget` _aswidget_component)))
      (return _aswb_info_frame))))

(fn `TurnLightGreenByTag`
  (params (Tag :type Name))
  (locals (SearchTag :type Name))
  (set `local.SearchTag` Tag)
  (for _array_element (`SceneComponent.GetChildrenComponents` (`self.Lights`) false)
    (if (== (`|GetArrayItem` (`ActorComponent.ComponentTags` _array_element)) (`local.SearchTag`))
      (bind _asstatic_mesh_component (cast `StaticMeshComponent` _array_element))
      (`PrimitiveComponent.SetMaterial` _asstatic_mesh_component 0 "/Game/Lewin/MI_GlowLight_Green.MI_GlowLight_Green")
      (bind _aspoint_light_component (cast `PointLightComponent` (`SceneComponent.GetChildComponent` _array_element 0)))
      (`LightComponent.SetLightColor` _aspoint_light_component (struct :`G` 0.098958 :`A` 1.0) true)
      (break))))

(fn `UserConstructionScript`)