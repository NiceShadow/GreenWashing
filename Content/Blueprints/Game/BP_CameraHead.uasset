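; BP_CameraHead is an interactable AI pawn with a hidden head bone and a camera mesh that flees the player when interacted with.
; On BeginPlay, physical animation drives simulated bodies below spine_01.
; Focus toggles custom depth on both meshes, and a getter exposes its interaction widget.
; Interaction runs AI MoveTo toward a random navigable point away from the player, with debug trace and prints.
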(event `self.ReceiveBeginPlay`
  ;[1 1 1] Event BeginPlay
  (`SkinnedMeshComponent.HideBoneByName` (`self.Mesh`) "head" "PBO_None")
  (`PhysicalAnimationComponent.SetSkeletalMeshComponent` (`self.PhysicalAnimation`) (`self.Mesh`))
  (`PhysicalAnimationComponent.ApplyPhysicalAnimationSettingsBelow` (`self.PhysicalAnimation`) "spine_01" (make `PhysicalAnimationData` true 1000.0 100.0 1000.0 100.0) false)
  (`SkeletalMeshComponent.SetAllBodiesBelowSimulatePhysics` (`self.Mesh`) "spine_01" true false))

(event `RunAway`
  (set `self.FoundTargetLoc` (`self.CalculateLocation`))
  ;[1 1 1] Debug Target Loc
  (`KismetSystemLibrary.LineTraceSingle` :`Start` (+ (`self.FoundTargetLoc`) (0.0 0.0 200.0)) :`End` (`self.FoundTargetLoc`) :`TraceChannel` "TraceTypeQuery1" :`DrawDebugType` "ForDuration" :`TraceColor` (struct :`R` 1.0 :`B` 0.91469 :`A` 1.0) :`TraceHitColor` (struct :`R` 0.086714 :`G` 0.17103 :`B` 0.265625 :`A` 1.0))
  (`|AIMoveTo` self (`self.FoundTargetLoc`) null
    (:`OnSuccess`
      (`KismetSystemLibrary.PrintString` "F" true true (struct :`G` 0.66 :`B` 1.0 :`A` 1.0) 1.0))
    (:`OnFail`
      (`KismetSystemLibrary.PrintString` "S" true true (struct :`G` 0.66 :`B` 1.0 :`A` 1.0) 1.0))))

(event `/Game/Interaction/BI_Interaction.Interface_ToggleFocus`
  (params (Focus :type Boolean))
  (`PrimitiveComponent.SetRenderCustomDepth` (`self.Mesh`) Focus)
  (`PrimitiveComponent.SetRenderCustomDepth` (`self.CameraMesh`) Focus))

(event `/Game/Interaction/BI_Interaction.InterfaceInteract`
  (`self.RunAway`))

(fn `CalculateLocation`
  (returns (Return :type "Vector Structure"))
  (bind _randomlocation (`NavigationSystemV1.K2_GetRandomLocationInNavigableRadius` (+ (* (`KismetMathLibrary.GetForwardVector` (`KismetMathLibrary.FindLookAtRotation` (`self.K2_GetActorLocation`) (`self.K2_GetActorLocation` (`GameplayStatics.GetPlayerCharacter` 0)))) -500.0) (`self.K2_GetActorLocation`)) 250.0 null null))
  (return _randomlocation))

(fn `GetInteractionWidgetRef`
  (returns (Ref :type "WidgetComponent Object Reference"))
  (return (`self.Widget`)))

(fn `UserConstructionScript`)