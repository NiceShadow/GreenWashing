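; Component on BP_FirstPersonCharacter that handles footstep, landing and car powerup feedback, caching its owner at BeginPlay.
; StartWalking runs a looping timer paced by FootstepRate that plays footsteps only while the character is on the ground.
; Each step, and each landing, spawns a sound below the owner, chosen by the surface state from ACFootstepsScanner.
; UsingCar updates the powerup UI and plays a driving sound; UsingJetpack is empty.
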(event `self.ReceiveBeginPlay`
  (`self.SetUp`))

(event `self.ReceiveTick`
  (params (DeltaSeconds :type "Float (single-precision)")))

(event `CheckPlayFootstepsSound`
  ;[1 1 1] FootstepSound
  (if (`NavMovementComponent.IsMovingOnGround` (`Character.CharacterMovement` (`self.ChararacterRef`)))
    (`self.PlayFootstepsSound`)))

(event `StartWalking`
  (params (Start :type Boolean))
  (bind _returnvalue (/ 1.0 (`self.FootstepRate`)))
  ;[1 1 1] FootstepSound
  (if Start
    (bind _returnvalue_2 (`KismetSystemLibrary.K2_SetTimerDelegate` (delegate `CheckPlayFootstepsSound`) (* _returnvalue 0.45) true (* _returnvalue -0.15)))
    (set `self.FootstepSoundTimer` _returnvalue_2)
    (else
      (`KismetSystemLibrary.K2_ClearAndInvalidateTimerHandle` (`self.FootstepSoundTimer`)))))

(event `PlayFootstepsSound`
  ;[1 1 1] FootstepSound
  (`GameplayStatics.SpawnSoundAtLocation` (select `/Game/Blueprints/Game/E_FootstepsState` (`/Game/Blueprints/Game/AC_FootstepsScanner.CurrentState` (`/Game/Blueprints/Game/BP_FirstPersonCharacter.AC_FootstepsScanner` (`self.ChararacterRef`))) :`NewEnumerator1` "/Game/Audio/MetaFotsteps_Concrete.MetaFotsteps_Concrete" :`NewEnumerator2` "/Game/Audio/MetaFotsteps_Metal.MetaFotsteps_Metal" :`NewEnumerator3` "/Game/Audio/MetaFotsteps_Grass.MetaFotsteps_Grass" :`NewEnumerator5` "/Game/Audio/MetaFotsteps_Carpet.MetaFotsteps_Carpet" :`NewEnumerator6` "/Game/Audio/MetaFotsteps_SoftMetal.MetaFotsteps_SoftMetal" :!type "SoundBase Object Reference") (- (`Actor.K2_GetActorLocation` (`self.GetOwner`)) (0.0 0.0 40.0)) (struct) 1.0 1.0 0.0 null null))

(event `EventOnLanded`
  ;[1 1 1] FootstepSound
  (`self.PlayFootstepsSound`))

(event `UsingCar`
  (params (in :type Boolean))
  ;[1 1 1] Use Powerups
  (`/Game/UI/Game/WB_UI.UsePowerup` (`/Game/Blueprints/Game/BP_GeneralFunctions.GetUI`) in (`self.CarDuration`))
  (if in
    (`GameplayStatics.SpawnSoundAtLocation` "/Game/Audio/DrivingCar.DrivingCar" (`Actor.K2_GetActorLocation` (`self.GetOwner`)) (struct) 1.0 1.0 0.0 null null)))

(event `UsingJetpack`
  (params (In :type Boolean))
  ;[1 1 1] Use Powerups
)

(fn `SetUp`
  (bind _asbp_first_person_character (cast `/Game/Blueprints/Game/BP_FirstPersonCharacter` (`self.GetOwner`)))
  (set `self.ChararacterRef` _asbp_first_person_character))