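; BP_GeneralFunctions is a set of shared getter functions for core player references.
; GetUI returns the UI reference held by BP_OurHUD, and GetCameraHeadRef returns the camera head reference held by BP_OurPlayerController.
; GetCharacterRef returns the player character as BP_FirstPersonCharacter.
; All three look up player index 0 and cast to the project class, so they only serve the first player.
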(fn `GetCameraHeadRef`
  (returns (CameraHeadRef :type "/Game/Blueprints/Game/BP_CameraHead Object Reference"))
  (bind _asbp_our_player_controller (cast `/Game/Blueprints/Game/BP_OurPlayerController` (`GameplayStatics.GetPlayerController` null)))
  (return (`/Game/Blueprints/Game/BP_OurPlayerController.CamHeadRef` _asbp_our_player_controller)))

(fn `GetCharacterRef`
  (returns (FP_Char :type "/Game/Blueprints/Game/BP_FirstPersonCharacter Object Reference"))
  (bind _asbp_first_person_character (cast `/Game/Blueprints/Game/BP_FirstPersonCharacter` (`GameplayStatics.GetPlayerCharacter` null)))
  (return _asbp_first_person_character))

(fn `GetUI`
  (returns (UI_Ref :type "/Game/UI/Game/WB_UI Object Reference"))
  (bind _asbp_our_hud (cast `/Game/Blueprints/Game/BP_OurHUD` (`PlayerController.GetHUD` (`GameplayStatics.GetPlayerController` null))))
  (return (`/Game/Blueprints/Game/BP_OurHUD.UI_Ref` _asbp_our_hud)))