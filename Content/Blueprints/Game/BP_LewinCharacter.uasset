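; BP_LewinCharacter handles Lewin's encounter with the Camera Head, which screaming can scare away.
; Focusing on it plays a sighting voice line until it has fled; Tick makes it run away when focus and screaming coincide.
; High noise before a valid scream triggers a brief scare reaction while focused.
; When screaming stops after it flees, a one-time follow-up line plays, delayed if the sighting line is still valid.
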(event `self.ReceiveTick`
  (params (DeltaSeconds :type "Float (single-precision)"))
  (if (`self.CamHeadFocused`)
    (if (`self.IsScreaming`)
      (`/Game/Blueprints/Game/BP_CameraHead.RunAway` (`/Game/Blueprints/Game/BP_GeneralFunctions.GetCameraHeadRef`) true)
      (set `self.CamHeadRanAwayAlready` true))))

(event `DetectedScream`
  (params (In :type Boolean))
  (bind _output_get (set `self.IsScreaming` In))
  (`KismetSystemLibrary.PrintString` (`KismetStringLibrary.Conv_BoolToString` In) true true (struct :`R` 0.913823 :`G` 1.0 :`A` 1.0))
  (if _output_get
    _
    (elif (`self.CamHeadRanAwayAlready`)
      (`/Engine/EditorBlueprintResources/StandardMacros.DoOnce` false
        (:`Completed`
          (`/Engine/EditorBlueprintResources/StandardMacros.IsValid` (`self.VoiceLine1`)
            (:`Is Valid`
              (`KismetSystemLibrary.Delay` 4.0))
            (:`Is Not Valid`
              _))
          (`/Game/Blueprints/Game/BP_FirstPersonCharacter.PlayVoiceLines` (`/Game/Blueprints/Game/BP_GeneralFunctions.GetCharacterRef`) "/Game/Audio/AudioFiles/VoiceLines/AfterScreamingAtCameraHead.AfterScreamingAtCameraHead"))))))

(event `UsingCar`
  (params (in :type Boolean)))

(event `UsingJetpack`
  (params (In :type Boolean)))

(event `OnFocusCameraHead`
  (params (Focus :type Boolean))
  (bind _output_get (set `self.CamHeadFocused` Focus))
  (if _output_get
    (if (not (`self.CamHeadRanAwayAlready`))
      (`/Engine/EditorBlueprintResources/StandardMacros.IsValid` (`self.VoiceLine1`)
        (:`Is Not Valid`
          (bind _returnvalue (`/Game/Blueprints/Game/BP_FirstPersonCharacter.PlayVoiceLines` (`/Game/Blueprints/Game/BP_GeneralFunctions.GetCharacterRef`) "/Game/Audio/AudioFiles/VoiceLines/SeeCameraheadVoiceLine.SeeCameraheadVoiceLine"))
          (set `self.VoiceLine1` _returnvalue))))))

(event `PlayCH_Reaction`
  (set `/Game/Blueprints/Game/BP_FirstPersonCharacter.IsPlayingCH_Reaction` true (`/Game/Blueprints/Game/BP_GeneralFunctions.GetCharacterRef`))
  (`/Game/Blueprints/Game/BP_CameraHead.PlayScareReaction` (`/Game/Blueprints/Game/BP_GeneralFunctions.GetCameraHeadRef`))
  (`KismetSystemLibrary.Delay` 1.1)
  (set `/Game/Blueprints/Game/BP_FirstPersonCharacter.IsPlayingCH_Reaction` false (`/Game/Blueprints/Game/BP_GeneralFunctions.GetCharacterRef`)))

(fn `HighNoiseBeforeValidScreaming`
  (if (`self.CamHeadFocused`)
    (`self.PlayCH_Reaction`)))