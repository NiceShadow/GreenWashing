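; BP_InfoCollectible is an interactable info collectible built around a child BP_Projector, which outlines on focus.
; Its construction script pushes media, lens, light and state settings into the projector, so each instance previews its setup.
; The first interaction unlocks it, plays a level sequence and voice line, and notifies the info point by tag with a delayed light.
; Interacting also turns the projector on, depending on its state.
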(event `/Game/Interaction/BI_Interaction.InterfaceInteract`
  (`self.Unlock`)
  (`|ExecutionSequence`
    (:`then_0`
      (`/Engine/EditorBlueprintResources/StandardMacros.DoOnce` false
        (:`Completed`
          (`/Game/Blueprints/Game/BP_FirstPersonCharacter.PlayVoiceLines` (`/Game/Blueprints/Game/BP_GeneralFunctions.GetCharacterRef`) (`self.VoiceLineToPlay`)))))
    (:`then_1`
      (bind _asbp_projector (cast `/Game/Projector/BP_Projector` (`ChildActorComponent.ChildActor` (`self.Projector`))))
      (if (not (`|EnumEquality` (`/Game/Projector/BP_Projector.State` _asbp_projector) "NewEnumerator0"))
        (`/Game/Projector/BP_Projector.TurnOn` _asbp_projector)))))

(event `/Game/Interaction/BI_Interaction.Interface_ToggleFocus`
  (params (Focus :type Boolean) (Index :type Integer))
  (bind _asbp_projector (cast `/Game/Projector/BP_Projector` (`ChildActorComponent.ChildActor` (`self.Projector`))))
  (`/Game/Projector/BP_Projector.ShowOutline` _asbp_projector Focus))

(event `OnUnlucked`
  (`/Game/Blueprints/Game/BP_InfoPoint.CheckForInfo` (`self.InfoPointRef`) (`self.TagID`) true 3.0))

(fn `GetInteractionWidgetRef`
  (returns (Ref :type "WidgetComponent Object Reference"))
  (return (`self.Widget`)))

(fn `Unlock`
  (if (not (`self.Unlocked`))
    (set `self.Unlocked` true)
    (`self.OnUnlucked`)
    (bind (_outactor _returnvalue) (`LevelSequencePlayer.CreateLevelSequencePlayer` (`self.Level Sequence`)))
    (`MovieSceneSequencePlayer.Play` _returnvalue)))

(fn `UserConstructionScript`
  (bind _asbp_projector (cast `/Game/Projector/BP_Projector` (`ChildActorComponent.ChildActor` (`self.Projector`))))
  (set `/Game/Projector/BP_Projector.Projected Media` (`self.Projected Media`) _asbp_projector)
  (set `/Game/Projector/BP_Projector.Attenuation Radius` (`self.Attenuation Radius`) _asbp_projector)
  (set `/Game/Projector/BP_Projector.Vertical Lens Shift` (`self.VerticalShift`) _asbp_projector)
  (set `/Game/Projector/BP_Projector.Horizontal Lens Shift` (`self.HorizontalShift`) _asbp_projector)
  (`/Game/Projector/BP_Projector.SetThrowRatio` _asbp_projector (`self.Throw Ratio`))
  (set `/Game/Projector/BP_Projector.Light Intensity` (`self.Light Intensity`) _asbp_projector)
  (set `/Game/Projector/BP_Projector.Image Resolution` (`self.Image Resolution`) _asbp_projector)
  (`/Game/Projector/BP_Projector.Update Image` _asbp_projector)
  (set `/Game/Projector/BP_Projector.State` (`self.State`) _asbp_projector)
  (`/Game/Projector/BP_Projector.Set Initial Projector State` _asbp_projector)
  (`/Game/Projector/BP_Projector.Set Up Light Textures` _asbp_projector)
  (`/Game/Projector/BP_Projector.Set Up Light Parameters` _asbp_projector)
  (`/Game/Projector/BP_Projector.Set Up Projector Parameters` _asbp_projector))