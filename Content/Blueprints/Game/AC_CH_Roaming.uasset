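; Actor component for BP_CameraHead that makes it wander when it has not been running away for a while.
; Tick counts up while the character is calm, starting a walk to a random nearby point at a threshold; running away resets roaming.
; WalkAgainInAFewSec sets a random standing pause, which Tick counts down before requesting the next walk.
; Counters named as seconds increment once per tick, and all logic halts during the winning final cutscene.
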(event `self.ReceiveBeginPlay`
  (bind _asbp_camera_head (cast `/Game/Blueprints/Game/BP_CameraHead` (`self.GetOwner`)))
  (set `self.chREF` _asbp_camera_head))

(event `self.ReceiveTick`
  (params (DeltaSeconds :type "Float (single-precision)"))
  (if (`/Game/Blueprints/Game/BP_OurPlayerController.WON_FinalCutscene` (`/Game/Blueprints/Game/BP_GeneralFunctions.GetPC`))
    _
    (elif (`/Game/Blueprints/Game/BP_CameraHead.CurrentlyRunningAway` (`self.chREF`))
      (set `self.SecondsNoScream` 0)
      (set `self.WaitToWalkAgain` false)
      (set `self.WaitSecToWalk` 0)
      (set `self.Roaming` false)
      (else
        (`|ExecutionSequence`
          (:`then_0`
            (bind _result (`/Engine/EditorBlueprintResources/StandardMacros.IncrementInt` (`self.SecondsNoScream`))
              (:`  `
                (if (>= _result 12)
                  (if (not (`self.Roaming`))
                    (set `self.Roaming` true)
                    (`/Game/Blueprints/Game/BP_CameraHead.WalkToRandomNearbyPoint` (`self.chREF`)))))))
          (:`then_1`
            (if (`self.WaitToWalkAgain`)
              (bind _result_2 (`/Engine/EditorBlueprintResources/StandardMacros.IncrementInt` (`self.WaitSecToWalk`))
                (:`  `
                  (if (>= _result_2 (`self.RandomStanding`))
                    (set `self.WaitToWalkAgain` false)
                    (set `self.WaitSecToWalk` 0)
                    (`/Game/Blueprints/Game/BP_CameraHead.WalkToRandomNearbyPoint` (`self.chREF`))))))))))))

(event `WalkAgainInAFewSec`
  (if (not (`/Game/Blueprints/Game/BP_OurPlayerController.WON_FinalCutscene` (`/Game/Blueprints/Game/BP_GeneralFunctions.GetPC`)))
    (set `self.WaitToWalkAgain` true)
    (set `self.RandomStanding` (`KismetMathLibrary.RandomIntegerInRange` 2 7))))