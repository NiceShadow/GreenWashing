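; Actor component that detects the surface under its owner and reports it as a footstep state.
; Each tick it runs a downward multi sphere trace and maps the first hit's physical material name to a surface enum, with a default for misses or unknown materials.
; CheckForNewState calls the FootstepsStateChanged dispatcher only when that state changes, and prints the new value to screen.
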(event `self.ReceiveTick`
  (params (DeltaSeconds :type "Float (single-precision)"))
  (bind _returnvalue (`Actor.K2_GetActorLocation` (`self.GetOwner`)))
  (bind (_outhits _returnvalue_2) (`KismetSystemLibrary.SphereTraceMulti` (+ _returnvalue (0.0 0.0 -50.0)) (- _returnvalue (0.0 0.0 200.0)) 50.0 "TraceTypeQuery4"))
  (if _returnvalue_2
    (switch `string` (`KismetSystemLibrary.GetDisplayName` (`.PhysMat` (`GameplayStatics.BreakHitResult` (`|GetArrayItem` _outhits))))
      (:`Default`
        (set `self.FoundState` "NewEnumerator0"))
      (:`PM_Concrete`
        (set `self.FoundState` "NewEnumerator1"))
      (:`PM_Metal`
        (set `self.FoundState` "NewEnumerator2"))
      (:`PM_Soil`
        (set `self.FoundState` "NewEnumerator3"))
      (:`PM_ThisMaterialInParks`
        (set `self.FoundState` "NewEnumerator5"))
      (:`PM_Wood`
        (set `self.FoundState` "NewEnumerator4")))
    (`self.CheckForNewState`)
    (else
      (set `self.FoundState` "NewEnumerator0")
      (`self.CheckForNewState`))))

(fn `CheckForNewState`
  (if (`|EnumInequality` (`self.CurrentState`) (`self.FoundState`))
    (bind _output_get (set `self.CurrentState` (`self.FoundState`)))
    (`self.FootstepsStateChanged` _output_get)
    (`KismetSystemLibrary.PrintString` (`|GetEnumeratorNameAsString` _output_get))))