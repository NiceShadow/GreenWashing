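; BP_MenuPC is a player controller for the menu, setting UI-only input with a visible mouse cursor on BeginPlay.
; It also initializes the Simple Controller target for gamepad input and binds events for button presses and the directional pad.
; Both handlers switch on the incoming value but have no actions wired to any case.
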(event `self.ReceiveBeginPlay`
  (`WidgetBlueprintLibrary.SetInputMode_UIOnlyEx` self null)
  (set `self.bShowMouseCursor` true)
  (`SimpleControllerBPLibrary.initController` (`SimpleControllerBPLibrary.getSimpleControllerTarget`) "Index_60" false true)
  (add `SimpleControllerBPLibrary.onButtonDownEventDelegate` (`SimpleControllerBPLibrary.getSimpleControllerTarget`) (delegate `onButtonDownEventDelegate_Event_1`))
  (add `SimpleControllerBPLibrary.onDirectionalPadEventDelegate` (`SimpleControllerBPLibrary.getSimpleControllerTarget`) (delegate `onDirectionalPadEventDelegate_Event_0`)))

(event `onButtonDownEventDelegate_Event_1`
  (params (deviceID :type String) (buttonID :type Integer) (deviceIndex :type Integer) (device :type "SimpleControllerDevice Structure"))
  (switch `int` buttonID))

(event `onDirectionalPadEventDelegate_Event_0`
  (params (deviceID :type String) (directionalPadValue :type Integer) (directionalPadIndex :type Integer) (deviceIndex :type Integer) (device :type "SimpleControllerDevice Structure"))
  (switch `int` directionalPadValue))

(fn `UserConstructionScript`)