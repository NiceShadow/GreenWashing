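; BP_Kai is an actor that plays a video through a child BP_Projector with sound and animates a flag mesh.
; On BeginPlay it hides the projector mesh, and its PlayVideo event starts the projector and media sound.
; Animate reveals the flag, stretches its Y scale with a timeline, then assigns it to InterpToMovement.
; Nothing in this Blueprint's live logic calls either event.
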(event `self.ReceiveBeginPlay`
  (bind _asbp_projector (cast `/Game/Projector/BP_Projector` (`ChildActorComponent.ChildActor` (`self.Projector`))))
  (`SceneComponent.SetHiddenInGame` (`/Game/Projector/BP_Projector.ProjectorMesh` _asbp_projector) true false))

(event `PlayVideo`
  (bind _mediasound (`self.MediaSound`))
  (bind _asbp_projector (cast `/Game/Projector/BP_Projector` (`ChildActorComponent.ChildActor` (`self.Projector`))))
  (`/Game/Projector/BP_Projector.Play` _asbp_projector)
  (`SynthComponent.Start` _mediasound)
  (`SynthComponent.SetVolumeMultiplier` _mediasound 1.4))

(event `Animate`
  (`SceneComponent.SetHiddenInGame` (`self.flagtest2`) false false)
  (`TimelineComponent.SetPlayRate` (`self.Timeline_0`) 0.7)
  (bind (_direction _newtrack_0) (`Timeline|Timeline_0` :!via `PlayFromStart`)
    (:`Update`
      (`SceneComponent.SetRelativeScale3D` (`self.flagtest2`) (`KismetMathLibrary.MakeVector` 1.0 (`KismetMathLibrary.Lerp` 0.032966 1.0 _newtrack_0) 1.0)))
    (:`Finished`
      (`MovementComponent.SetUpdatedComponent` (`self.InterpToMovement`) (`self.flagtest2`)))))

(fn `UserConstructionScript`)