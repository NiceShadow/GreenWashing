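; BP_InteractionArea_Master is an interaction area that relays focus changes to the parent actor it is attached to as a child actor.
; ToggleFocus stores the focus state and sends it with the area's index to the parent through a message call.
; It then requests the parent's interaction widget and, if valid, shows it while focused and hides it otherwise.
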(event `ToggleFocus`
  (params (Focused :type Boolean))
  (set `self.Focused` Focused)
  (message `/Game/Interaction/BI_Interaction.Interface_ToggleFocus` (`self.GetParentActor`) (`self.Focused`) (`self.Index`))
  (bind _ref (message `/Game/Interaction/BI_Interaction.GetInteractionWidgetRef` (`self.GetParentActor`)))
  (`/Engine/EditorBlueprintResources/StandardMacros.IsValid` _ref
    (:`Is Valid`
      (`SceneComponent.SetHiddenInGame` _ref (not (`self.Focused`)) false))))

(fn `UserConstructionScript`)