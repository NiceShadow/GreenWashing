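; Player interaction component that finds, highlights and triggers interaction areas under the camera.
; Each tick it line-traces from the camera, capped at 500 units unless the actor's first tag is "longer", focusing only BP_InteractionArea_CustomShape hits.
; Interact input sends an interface message to the area's parent actor through InteractOnServer.
; Special cases notify the character of camera-head focus and, for cars, stop tracing, call UseCar and destroy the car.
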(event `self.ReceiveTick`
  (params (DeltaSeconds :type "Float (single-precision)"))
  (`self.Trace`))

(event `TryToInteract`
  (params (In :type Boolean))
  (if In
    (if (`self.IsTracingInteractionArea`)
      (`self.InteractOnServer` (`self.FocusedInteractionArea`))
      (`self.GetParentActorAndCheckForEvent`))))

(event `InteractOnServer`
  (params (InteractionArea :type "/Game/Interaction/InteractionArea/BP_InteractionArea_Master Object Reference"))
  (message `/Game/Interaction/BI_Interaction.InterfaceInteract` (`Actor.GetParentActor` InteractionArea)))

(fn `GetParentActorAndCheckForEvent`
  (locals (ParentActor :type "Actor Object Reference"))
  (bind _output_get (set `local.ParentActor` (`Actor.GetParentActor` (`self.FocusedInteractionArea`))))
  (if (== (`GameplayStatics.GetObjectClass` _output_get) "/Game/Blueprints/Game/BP_Car.BP_Car_C")
    (set `self.StopTracing` true)
    (bind _asbp_first_person_character (cast `/Game/Blueprints/Game/BP_FirstPersonCharacter` (`self.GetOwner`)))
    (`/Game/Blueprints/Game/BP_FirstPersonCharacter.UseCar` _asbp_first_person_character)
    (`Actor.K2_DestroyActor` (`local.ParentActor`))))

(fn `StopInteraction`)

(fn `Trace`
  (bind _returnvalue (`GameplayStatics.GetPlayerCameraManager` 0))
  (bind _returnvalue_2 (`Actor.K2_GetActorLocation` _returnvalue))
  (if (`self.StopTracing`)
    (`self.TraceInteractionArea` false)
    (else
      (bind (_outhit _returnvalue_3) (`KismetSystemLibrary.LineTraceSingle` _returnvalue_2 (+ _returnvalue_2 (* (`KismetMathLibrary.GetForwardVector` (`PlayerCameraManager.GetCameraRotation` _returnvalue)) (`self.Length`))) "TraceTypeQuery1"))
      (if _returnvalue_3
        (bind (_bblockinghit _binitialoverlap _time _distance _location _impactpoint _normal _impactnormal _physmat _hitactor) (`GameplayStatics.BreakHitResult` _outhit))
        (bind _tags (`Actor.Tags` _hitactor))
        (if (> (`KismetArrayLibrary.Array_Length` _tags) 0)
          (if (== (`|GetArrayItem` _tags) "longer")
            (if (!= (`self.FocusedActor`) _hitactor) :!label _label
              (set `self.FocusedActor` _hitactor)
              (`self.TraceInteractionArea` (== (`GameplayStatics.GetObjectClass` _hitactor) "/Game/Interaction/InteractionArea/BP_InteractionArea_CustomShape.BP_InteractionArea_CustomShape_C")))
            (else
              (if (< _distance 500.0) :!label _label_2
                (goto _label)
                (else
                  (`self.TraceInteractionArea` false :!label _label_3)))))
          (else
            (goto _label_2)))
        (else
          (goto _label_3))))))

(fn `TraceInteractionArea`
  (params (Trace :type Boolean))
  (bind _focusedinteractionarea (`self.FocusedInteractionArea`))
  (if Trace
    (if (`self.IsTracingInteractionArea`)
      (`/Game/Interaction/InteractionArea/BP_InteractionArea_Master.ToggleFocus` (`self.FocusedInteractionArea`) false))
    (bind _asbp_interaction_area_master (cast `/Game/Interaction/InteractionArea/BP_InteractionArea_Master` (`self.FocusedActor`)))
    (bind _output_get (set `self.FocusedInteractionArea` _asbp_interaction_area_master))
    (`/Game/Interaction/InteractionArea/BP_InteractionArea_Master.ToggleFocus` _output_get true)
    (set `self.IsTracingInteractionArea` true)
    (if (== (`GameplayStatics.GetObjectClass` (`Actor.GetParentActor` (`self.FocusedInteractionArea`))) "/Game/Blueprints/Game/BP_CameraHead.BP_CameraHead_C")
      (`/Game/Blueprints/Game/BP_LewinCharacter.OnFocusCameraHead` (`/Game/Blueprints/Game/BP_FirstPersonCharacter.BP_LewinCharacter` (`/Game/Blueprints/Game/BP_GeneralFunctions.GetCharacterRef`)) true))
    (elif (`self.IsTracingInteractionArea`)
      (set `self.IsTracingInteractionArea` false)
      (`/Engine/EditorBlueprintResources/StandardMacros.IsValid` _focusedinteractionarea
        (:`Is Valid`
          (`/Game/Interaction/InteractionArea/BP_InteractionArea_Master.ToggleFocus` _focusedinteractionarea false)
          (if (== (`GameplayStatics.GetObjectClass` (`Actor.GetParentActor` _focusedinteractionarea)) "/Game/Blueprints/Game/BP_CameraHead.BP_CameraHead_C")
            (`/Game/Blueprints/Game/BP_LewinCharacter.OnFocusCameraHead` (`/Game/Blueprints/Game/BP_FirstPersonCharacter.BP_LewinCharacter` (`/Game/Blueprints/Game/BP_GeneralFunctions.GetCharacterRef`)) false))
          (set `self.FocusedActor` null)
          (set `self.FocusedInteractionArea` null))
        (:`Is Not Valid`
          (set `self.FocusedActor` null))))))